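; BP_Cat is an animated cat that moves forward over a set path length, then disappears with a burst effect and sound.
; Tick moves the mesh at CurrentSpeed and counts down PathLength.
; A looping timer briefly switches walking speed to SecondSpeed, scaling animation play rate to match; per comments, BP_House supplies the speeds.
; A slower timer detects arrival, then hides the cat and destroys it after a delay.
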(event `CheckPathLength`
  (if (< (`self.PathLength`) 0.0)
    (`/Engine/EditorBlueprintResources/StandardMacros.DoOnce` false
      (:`Completed`
        (`|ExecutionSequence`
          (:`then_0`
            ;[0.09896 0.09896 0.09896 1 14] Repeat DirectionalBurst
            (`SceneComponent.K2_SetRelativeTransform` (`self.NS_DirectionalBurst`) (`KismetMathLibrary.MakeTransform` (-20.0 0.0 10.0) (struct :`Pitch` 30.0 :`Yaw` 180.0)) false false)
            (`ActorComponent.Activate` (`self.NS_DirectionalBurst`) false)
            (`AddComponent|NODE_AddAudioComponent-0`) ; Play Sound on Arrival
          )
          (:`then_1`
            ;[0.09896 0.09896 0.09896 1 14] Remove Cat
            (`SceneComponent.SetHiddenInGame` (`self.SkeletalMesh`) true false)
            (`self.SetActorTickEnabled` false)
            (`KismetSystemLibrary.Delay` 2.0)
            (`self.K2_DestroyActor`)))))))

(event `self.ReceiveBeginPlay`
  (bind _secondduration (`self.SecondDuration`))
  (`|ExecutionSequence`
    (:`then_0`
      (`SkeletalMeshComponent.PlayAnimation` (`self.SkeletalMesh`) "/Game/Cat/A_Cat.A_Cat" true)
      (`AddComponent|NODE_AddAudioComponent-1`) ; Play Sound on Spawn
    )
    (:`then_1`
      ;[0.1615 0.1615 0.1615] CurrentSpeed Toggling with Timer and speed values from BP_House
      (`KismetSystemLibrary.K2_SetTimerDelegate` (delegate `ToggleMode`) (+ (`self.WalkingDuration`) _secondduration) true (* _secondduration -1.0)) ; every 1.5s with -0.5s delay => on 1.0, 2.5, 4, etc.
      (`self.UseWalkingSpeed` :!pinned true) ; Set CurrentSpeed to WalkingSpeed
      (`KismetSystemLibrary.K2_SetTimerDelegate` (delegate `CheckPathLength`) 0.1 true) ; Less often than Tick
    )))

(event `ToggleMode`
  ;[0.1615 0.1615 0.1615] CurrentSpeed Toggling with Timer and speed values from BP_House
  (`|ExecutionSequence`
    (:`then_0`
      (bind _output_get (set `self.currentSpeed` (`self.SecondSpeed`)))
      (`SkeletalMeshComponent.SetPlayRate` (`self.SkeletalMesh`) (/ _output_get 35.0)))
    (:`then_1`
      (`KismetSystemLibrary.Delay` (`self.SecondDuration`))
      (bind _output_get_2 (set `self.currentSpeed` (`self.WalkingSpeed`) :!label _label))
      (`SkeletalMeshComponent.SetPlayRate` (`self.SkeletalMesh`) (/ _output_get_2 35.0)))))

(event `UseWalkingSpeed`
  ;[0.1615 0.1615 0.1615] CurrentSpeed Toggling with Timer and speed values from BP_House
  (goto _label))

(event `self.ReceiveTick`
  (params (DeltaSeconds :type "Float (single-precision)"))
  (bind _returnvalue (* DeltaSeconds (`self.currentSpeed`)))
  (set `self.PathLength` (- (`self.PathLength`) _returnvalue))
  (`SceneComponent.K2_AddLocalTransform` (`self.SkeletalMesh`) (`KismetMathLibrary.MakeTransform` (`KismetMathLibrary.MakeVector` _returnvalue)) false false :!pinned true) ; Move with CurrentSpeed
)

(fn `UserConstructionScript`)