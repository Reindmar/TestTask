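; A one-shot button actor that glows per state and triggers a spawn on its linked Nest when pressed.
; The construction script creates a dynamic material instance for the cube, sets the unhovered emissive color and writes the label text.
; Hover, unhover and press events recolor the emissive parameter, and the first press also sinks the button and locks out further changes.
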(event `/Game/Blueprints/BPI_Interactable.Hovered`
  (if (not (`self.bPressed`))
    (`MaterialInstanceDynamic.SetVectorParameterValue` (`self.MI_Button`) "ButtonEmissive" (`self.HoveredColor`))))

(event `/Game/Blueprints/BPI_Interactable.Unhovered`
  (if (not (`self.bPressed`))
    (`MaterialInstanceDynamic.SetVectorParameterValue` (`self.MI_Button`) "ButtonEmissive" (`self.UnhoveredColor`))))

(event `/Game/Blueprints/BPI_Interactable.Pressed`
  (if (not (`self.bPressed`))
    (`MaterialInstanceDynamic.SetVectorParameterValue` (`self.MI_Button`) "ButtonEmissive" (`self.PressedColor`))
    (set `self.bPressed` true)
    (`SceneComponent.K2_AddLocalOffset` (`self.DefaultSceneRoot`) (0.0 0.0 -2.0) false false)
    (`/Game/Blueprints/BP_House.Spawn` (`self.Nest`) :!pinned true) ; Button Purpose
  ))

(fn `UserConstructionScript`
  (bind _returnvalue (`KismetMaterialLibrary.CreateDynamicMaterialInstance` (`self.M_Button`)))
  (bind _output_get (set `self.MI_Button` _returnvalue))
  (`MaterialInstanceDynamic.SetVectorParameterValue` _output_get "ButtonEmissive" (`self.UnhoveredColor`))
  (`PrimitiveComponent.SetMaterial` (`self.Cube`) 0 (`self.MI_Button`))
  (`TextRenderComponent.K2_SetText` (`self.ButtonName`) (`self.Name`)))