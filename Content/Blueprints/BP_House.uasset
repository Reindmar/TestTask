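; BP_House is a cat spawner with a DestinationHouse component marking the end of the path.
; Its construction script sets DestinationHouse's relative X position from PathLength, so the endpoint follows that variable.
; The Spawn event creates a BP_Cat at the root's location and rotation, passing it the path length and two speed and duration pairs.
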(event `Spawn`
  (bind _root (`self.Root`))
  (`|SpawnActorFromClass` "/Game/Blueprints/BP_Cat.BP_Cat_C" (`KismetMathLibrary.MakeTransform` (`SceneComponent.K2_GetComponentLocation` _root) (`SceneComponent.K2_GetComponentRotation` _root)) "Undefined" "OverrideRootScale" null (`self.PathLength`) (`self.WalkingSpeed`) (`self.WalkingDuration`) (`self.SecondSpeed`) (`self.SecondDuration`) null))

(fn `UserConstructionScript`
  (`SceneComponent.K2_SetRelativeLocation` (`self.DestinationHouse`) (`KismetMathLibrary.MakeVector` (`self.PathLength`)) false false))