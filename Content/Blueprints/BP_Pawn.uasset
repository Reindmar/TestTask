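; BP_Pawn is a player pawn that lets the player hover and click interactable actors through a crosshair-style camera trace.
; BeginPlay adds an audio component and the WBP_Pointer HUD widget.
; Each Tick traces forward from the camera and sends hovered, unhovered or left-click pressed messages to BPI_Interactable actors, tracking the last one hovered.
; The first successful press also starts a song, gated by DoOnce.
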(event `self.ReceiveBeginPlay`
  (`AddComponent|NODE_AddAudioComponent-0`)
  ;[0.09896 0.09896 0.09896 1 14] HUD
  (bind _returnvalue (`|GenericCreateObject` "/Game/Blueprints/WBP_Pointer.WBP_Pointer_C" self))
  (`UserWidget.AddToViewport` _returnvalue 0))

(event `self.ReceiveTick`
  (params (DeltaSeconds :type "Float (single-precision)"))
  (bind _transformcomponent (`PlayerCameraManager.TransformComponent` (`GameplayStatics.GetPlayerCameraManager` 0)))
  (bind _returnvalue (`SceneComponent.K2_GetComponentLocation` _transformcomponent))
  (bind _outhit (`KismetSystemLibrary.LineTraceSingle` _returnvalue (+ _returnvalue (* (`SceneComponent.GetForwardVector` _transformcomponent) 1000.0)) "TraceTypeQuery1" true))
  (if (`KismetSystemLibrary.DoesImplementInterface` (`.HitActor` (`GameplayStatics.BreakHitResult` _outhit)) "/Game/Blueprints/BPI_Interactable.BPI_Interactable_C") :!pinned true
    (if (not (== (`self.LastHovered`) (`.HitActor` (`GameplayStatics.BreakHitResult` _outhit)))) :!pinned true
      (message `/Game/Blueprints/BPI_Interactable.Unhovered` (`self.LastHovered`))
      (bind _output_get (set `self.LastHovered` (`.HitActor` (`GameplayStatics.BreakHitResult` _outhit)))))
    (if (`PlayerController.WasInputKeyJustPressed` (`GameplayStatics.GetPlayerController` 0) "LeftMouseButton") :!pinned true
      (message `/Game/Blueprints/BPI_Interactable.Pressed` _output_get)
      (`/Engine/EditorBlueprintResources/StandardMacros.DoOnce` false
        (:`Completed`
          (`AddComponent|NODE_AddAudioComponent-1`) ; Play song for first button
        ))
      (else
        (message `/Game/Blueprints/BPI_Interactable.Hovered` _output_get)))
    (else
      (message `/Game/Blueprints/BPI_Interactable.Unhovered` (`self.LastHovered`)))))

(fn `UserConstructionScript`)